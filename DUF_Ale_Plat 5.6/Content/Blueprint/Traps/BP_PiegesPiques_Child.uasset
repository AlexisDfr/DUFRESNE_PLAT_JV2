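; Spike trap actor, a child Blueprint that moves its spikes and hurts the third-person player character on contact.
; On BeginPlay, a timeline lerps the PiegesPiques component's relative location from the origin to NewPosition.
; Actor overlap subtracts one HP from BP_ThirdPersonCharacter and pushes the new health ratio to its UI.
; Parent BeginPlay and overlap calls are disabled, so this logic replaces the inherited behavior.
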(event Collision|EventActorBeginOverlap
  (params (OtherActor :type Actor%20Object%20Reference))
  (bind _asbp_third_person_character (Utilities|Casting|CastToBP_ThirdPersonCharacter OtherActor))
  (Variables|/Game/Blueprint/ThirdPerson/Blueprints/BP_ThirdPersonCharacter.BP_ThirdPersonCharacter_C|SetHP _asbp_third_person_character (- (Variables|/Game/Blueprint/ThirdPerson/Blueprints/BP_ThirdPersonCharacter.BP_ThirdPersonCharacter_C|GetHP _asbp_third_person_character) 1))
  (Default|SetPlayerHp (Variables|/Game/Blueprint/ThirdPerson/Blueprints/BP_ThirdPersonCharacter.BP_ThirdPersonCharacter_C|GetUI _asbp_third_person_character) (/ (Variables|/Game/Blueprint/ThirdPerson/Blueprints/BP_ThirdPersonCharacter.BP_ThirdPersonCharacter_C|GetHP _asbp_third_person_character) (Variables|/Game/Blueprint/ThirdPerson/Blueprints/BP_ThirdPersonCharacter.BP_ThirdPersonCharacter_C|GetHPMAX _asbp_third_person_character))))

(event EventTick
  (params (DeltaSeconds :type Float%20%28single-precision%29))
  (|CallParentFunction DeltaSeconds) ; This node is disabled and will not be called.\nDrag off pins to build functionality.
)

(event EventBeginPlay
  (bind _time (Timeline|Timeline_0 Play)
    (:Update
      (Transformation|SetRelativeLocation (Variables|Default|GetPiegesPiques) (Math|Vector|Lerp(Vector) "0, 0, 0" (Variables|Default|GetNewPosition) _time) false false))))

(fn ConstructionScript
  (|CallParentFunction))