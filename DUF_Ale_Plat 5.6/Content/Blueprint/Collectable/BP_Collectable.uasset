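; BP_Collectable is a health pickup that restores one HP to the third-person player character on overlap.
; On actor overlap it casts to BP_ThirdPersonCharacter and acts only if HP is below HPMAX.
; It then adds the health, pushes the new HP ratio to the character's UI and destroys itself, so it stays in the world when health is full.
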(event Collision|EventActorBeginOverlap
  (params (OtherActor :type Actor%20Object%20Reference))
  (bind _asbp_third_person_character (Utilities|Casting|CastToBP_ThirdPersonCharacter OtherActor))
  (if (< (Variables|/Game/LevelPrototyping/ThirdPerson/Blueprints/BP_ThirdPersonCharacter.BP_ThirdPersonCharacter_C|GetHP _asbp_third_person_character) (Variables|/Game/LevelPrototyping/ThirdPerson/Blueprints/BP_ThirdPersonCharacter.BP_ThirdPersonCharacter_C|GetHPMAX _asbp_third_person_character))
    (Variables|/Game/LevelPrototyping/ThirdPerson/Blueprints/BP_ThirdPersonCharacter.BP_ThirdPersonCharacter_C|SetHP _asbp_third_person_character (+ (Variables|/Game/LevelPrototyping/ThirdPerson/Blueprints/BP_ThirdPersonCharacter.BP_ThirdPersonCharacter_C|GetHP _asbp_third_person_character) 1))
    (Default|SetPlayerHp (Variables|/Game/LevelPrototyping/ThirdPerson/Blueprints/BP_ThirdPersonCharacter.BP_ThirdPersonCharacter_C|GetUI _asbp_third_person_character) (/ (Variables|/Game/LevelPrototyping/ThirdPerson/Blueprints/BP_ThirdPersonCharacter.BP_ThirdPersonCharacter_C|GetHP _asbp_third_person_character) (Variables|/Game/LevelPrototyping/ThirdPerson/Blueprints/BP_ThirdPersonCharacter.BP_ThirdPersonCharacter_C|GetHPMAX _asbp_third_person_character)))
    (Actor|DestroyActor)))

(fn ConstructionScript)